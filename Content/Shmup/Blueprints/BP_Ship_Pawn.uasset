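; BP_Ship_Pawn is the player's ship pawn in a shmup, handling movement, banking and shooting.
; Forward and right axis inputs, each gated by an enable flag, offset the actor without sweep along control-yaw directions.
; Sideways input also interpolates SceneRotation toward a roll angle, snapping it to zero when that input is zero.
; Pressing Shoot spawns a BP_Bullet_Base at ProjectilePoint and plays a 2D laser sound.
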(event EventBeginPlay
  (Utilities|FlowControl|Sequence
    (:then_0
      (Input|EnableInput 0))))

(event Collision|EventActorBeginOverlap
  (params (OtherActor :type Actor%20Object%20Reference)))

(event EventTick
  (params (DeltaSeconds :type Float%20%28single-precision%29)))

(event Input|ActionEvents|InputActionShoot
  (params (Key :type Key%20Structure))
  ;[1 1 1] Shooting
  (:Pressed
    (Game|SpawnActorfromClass "/Game/Shmup/Blueprints/BP_Bullet_Base.BP_Bullet_Base_C" (Transformation|GetWorldTransform (Variables|Default|GetProjectilePoint)) "Undefined" 0 0)
    (Audio|SpawnSound2D "/Game/Shmup/Audio/Ship_Laser_shoot_02.Ship_Laser_shoot_02" 1.0 1.0 0.0 0)))

(event Input|AxisEvents|InputAxisMoveForward
  (params (AxisValue :type Float%20%28single-precision%29))
  ;[1 1 1] Movement
  (if (Variables|Default|GetEnableMoveForward)
    (Transformation|AddActorWorldOffset (* (* (Math|Vector|GetForwardVector (Math|Rotator|MakeRotator 0.0 0.0 (.Yaw (Math|Rotator|BreakRotator (Pawn|GetControlRotation :!class /Script/Engine.Pawn))))) AxisValue) (Variables|Default|GetPlayerMoveRate)))))

(event Input|AxisEvents|InputAxisMoveRight
  (params (AxisValue :type Float%20%28single-precision%29))
  (bind _rollamount (Variables|Default|GetRollAmount))
  (bind _returnvalue (* AxisValue _rollamount))
  ;[1 1 1] Movement
  (if (Variables|Default|GetEnableMoveRight)
    (Transformation|AddActorWorldOffset (* (* (Math|Vector|GetRightVector (Math|Rotator|MakeRotator 0.0 0.0 (.Yaw (Math|Rotator|BreakRotator (Pawn|GetControlRotation :!class /Script/Engine.Pawn))))) AxisValue) (Variables|Default|GetPlayerMoveRate)))
    ;[1 1 1] Rotation
    (if (== _returnvalue 0.0)
      (Transformation|SetWorldRotation (Variables|Default|GetSceneRotation) (Math|Rotator|MakeRotator 0.0 0.0 0.0) false false)
      (else
        (Transformation|SetWorldRotation (Variables|Default|GetSceneRotation) (Math|Interpolation|RInterpTo (Transformation|GetWorldRotation (Variables|Default|GetSceneRotation)) (Math|Rotator|MakeRotator _returnvalue 0.0 0.0) (Utilities|Time|GetWorldDeltaSeconds) (Variables|Default|GetRollRate)) false false)))))

(fn ConstructionScript)