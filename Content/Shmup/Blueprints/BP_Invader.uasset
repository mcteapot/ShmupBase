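; BP_Invader is a shmup enemy that animates, moves along world X and breaks apart when shot.
; On BeginPlay it randomises scale and color, then runs timelines for limb animation (after a random delay) and movement, with direction set by MoveForward.
; A bullet overlapping its Box destroys the bullet, enables physics on the parts and sets IsShot, which Tick polls to stop both timelines.
; After a random delay it explodes with particles and sound.
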(event OnComponentBeginOverlap(Box)
  (params (OverlappedComponent :type Primitive%20Component%20Object%20Reference) (OtherActor :type Actor%20Object%20Reference) (OtherComp :type Primitive%20Component%20Object%20Reference) (OtherBodyIndex :type Integer) (bFromSweep :type Boolean) (SweepResult :type Hit%20Result%20Structure%20%28by%20ref%29))
  (bind _deathtimes (Variables|Default|GetDeathTimes))
  (bind _invader_body (Variables|Default|GetInvader_Body))
  (bind (_lowerbound _upperbound) (Utilities|Struct|BreakFloatRange _deathtimes))
  (bind _returnvalue (Transformation|GetWorldTransform _invader_body))
  (bind (_location _rotation) (Math|Transform|BreakTransform _returnvalue))
  ;[1 1 1] On Overlap
  (bind _asbp_bullet_base (Utilities|Casting|CastToBP_Bullet_Base OtherActor))
  (Default|BulletDestroy _asbp_bullet_base)
  (Audio|SpawnSound2D "/Game/Shmup/Audio/Invader_Explosion_01.Invader_Explosion_01")
  (Utilities|FlowControl|Sequence
    (:then_0
      ;[1 1 1] Enable Physics
      (for _array_element (Components|GetChildrenComponents (Variables|Default|GetArrow) false)
        (bind _asprimitive_component (Utilities|Casting|CastToPrimitiveComponent _array_element))
        (Physics|SetSimulatePhysics _asprimitive_component true)
        (Components|DestroyComponent (Variables|Default|GetBox))
        (Variables|Default|SetIsShot true)))
    (:then_1
      ;[1 1 1] Destroy Invader
      (Utilities|FlowControl|Delay (Math|Random|RandomFloatinRange (.Value (Utilities|Struct|BreakFloatRangeBound _lowerbound)) (.Value (Utilities|Struct|BreakFloatRangeBound _upperbound))))
      (Effects|SpawnEmitteratLocation "/Game/StarterContent/Particles/P_Explosion.P_Explosion" _location _rotation)
      (Audio|SpawnSound2D "/Game/Shmup/Audio/Invader_Explosion_02.Invader_Explosion_02")
      (Actor|DestroyActor))))

(event EventBeginPlay
  (bind _scalesizes (Variables|Default|GetScaleSizes))
  (bind _delaytimes (Variables|Default|GetDelayTimes))
  (bind (_lowerbound _upperbound) (Utilities|Struct|BreakFloatRange _scalesizes))
  (bind (_lowerbound_2 _upperbound_2) (Utilities|Struct|BreakFloatRange _delaytimes))
  (bind _value (Utilities|Struct|BreakFloatRangeBound _upperbound))
  (bind _value_2 (Utilities|Struct|BreakFloatRangeBound _lowerbound))
  (Utilities|FlowControl|Sequence
    (:then_0
      ;[1 1 1] Set Random Scale
      (Transformation|SetActorScale3D (Math|Vector|MakeVector (Math|Random|RandomFloatinRange _value_2 _value) (Math|Random|RandomFloatinRange _value_2 _value) (Math|Random|RandomFloatinRange _value_2 _value))))
    (:then_1
      ;[1 1 1] Set World Location Of Actor
      (Variables|Default|SetWordLocation (Transformation|GetActorLocation)))
    (:then_2
      ;[1 1 1] Start Delay
      (Utilities|FlowControl|Delay (Math|Random|RandomFloatinRange (.Value (Utilities|Struct|BreakFloatRangeBound _lowerbound_2)) (.Value (Utilities|Struct|BreakFloatRangeBound _upperbound_2))))
      ;[1 1 1] Animation Timeline
      (bind (_direction _armmove _legmove) (Timeline|Timeline_0 Play)
        (:Update
          (Utilities|FlowControl|Sequence
            (:then_0
              ;[1 1 1] Animation Arm
              (Transformation|SetRelativeLocation (Variables|Default|GetInvader_Arm_L) (Math|Vector|MakeVector 0.0 0.0 _armmove) false false))
            (:then_1
              (Transformation|SetRelativeLocation (Variables|Default|GetInvader_Arm_R) (Math|Vector|MakeVector 0.0 0.0 _armmove) false false))
            (:then_2
              ;[1 1 1] Animation Leg
              (Transformation|SetRelativeLocation (Variables|Default|GetInvader_Leg_L) (Math|Vector|MakeVector (stale _result) 0.0 0.0) false false))
            (:then_3
              (Transformation|SetRelativeLocation (Variables|Default|GetInvader_Leg_R) (Math|Vector|MakeVector _legmove 0.0 0.0) false false))))))
    (:then_3
      ;[1 1 1] Move Invader
      (bind _forward_move (Timeline|Timeline_1 Play)
        (:Update
          (if (Variables|Default|GetMoveForward)
            (Transformation|AddActorWorldOffset (Math|Vector|MakeVector _forward_move 0.0 0.0))
            (else
              (Transformation|AddActorWorldOffset (Math|Vector|NegateVector (Math|Vector|MakeVector _forward_move 0.0 0.0)))))
          (Variables|Default|SetWordLocation (Transformation|GetActorLocation)))))
    (:then_4
      ;[1 1 1] Set Random Color
      (Variables|Default|SetRandColor (Math|Vector|MakeVector (Math|Random|RandomFloatinRange 0.0 1.0) 0.0 (Math|Random|RandomFloatinRange 0.0 1.0))))
    (:then_5
      ;[1 1 1] Set Random Emissive
      (Variables|Default|SetRandEmissive (Math|Vector|MakeVector (Math|Random|RandomFloatinRange 0.0 1.0) 0.0 (Math|Random|RandomFloatinRange 0.0 1.0))))
    (:then_6
      ;[1 1 1] Apply Random Color
      (for _array_element (Components|GetChildrenComponents (Variables|Default|GetArrow) true)
        (bind _asmesh_component (Utilities|Casting|CastToMeshComponent _array_element))
        (Rendering|Material|SetVectorParameterValueonMaterials _asmesh_component "Color" (Variables|Default|GetRandColor))
        (Rendering|Material|SetVectorParameterValueonMaterials _asmesh_component "Emissive Color" (Variables|Default|GetRandColor))))))

(event Collision|EventActorBeginOverlap
  (params (OtherActor :type Actor%20Object%20Reference)))

(event EventTick
  (params (DeltaSeconds :type Float%20%28single-precision%29))
  (if (Variables|Default|GetIsShot)
    (Utilities|FlowControl|Sequence
      (:then_0
        ;[1 1 1] Move Invader
        (bind _forward_move (Timeline|Timeline_1 Stop)
          (:Update
            (if (Variables|Default|GetMoveForward)
              (Transformation|AddActorWorldOffset (Math|Vector|MakeVector _forward_move 0.0 0.0))
              (else
                (Transformation|AddActorWorldOffset (Math|Vector|NegateVector (Math|Vector|MakeVector _forward_move 0.0 0.0)))))
            (Variables|Default|SetWordLocation (Transformation|GetActorLocation)))))
      (:then_1
        ;[1 1 1] Animation Timeline
        (bind (_direction _armmove _legmove) (Timeline|Timeline_0 Stop)
          (:Update
            (Utilities|FlowControl|Sequence
              (:then_0
                ;[1 1 1] Animation Arm
                (Transformation|SetRelativeLocation (Variables|Default|GetInvader_Arm_L) (Math|Vector|MakeVector 0.0 0.0 _armmove) false false))
              (:then_1
                (Transformation|SetRelativeLocation (Variables|Default|GetInvader_Arm_R) (Math|Vector|MakeVector 0.0 0.0 _armmove) false false))
              (:then_2
                ;[1 1 1] Animation Leg
                (Transformation|SetRelativeLocation (Variables|Default|GetInvader_Leg_L) (Math|Vector|MakeVector (stale _result) 0.0 0.0) false false))
              (:then_3
                (Transformation|SetRelativeLocation (Variables|Default|GetInvader_Leg_R) (Math|Vector|MakeVector _legmove 0.0 0.0) false false)))))))))

(fn ConstructionScript)